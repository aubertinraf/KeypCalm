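; Short-lived projectile for the Fury Scream ability that breaks grabbable props it touches.
; It moves along its Direction by Speed each Tick without sweep, and a sphere overlap calls BreakProp on any BP_GrabProps it hits.
; A timer started at BeginPlay turns off the Niagara effect, then a second short timer destroys the actor.
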(event OnComponentBeginOverlap(Sphere)
  (params (OverlappedComponent :type Primitive%20Component%20Object%20Reference) (OtherActor :type Actor%20Object%20Reference) (OtherComp :type Primitive%20Component%20Object%20Reference) (OtherBodyIndex :type Integer) (bFromSweep :type Boolean) (SweepResult :type Hit%20Result%20Structure%20%28by%20ref%29))
  (bind _asbp_grab_props (Utilities|Casting|CastToBP_GrabProps OtherActor))
  (Default|BreakProp _asbp_grab_props))

(event EventTick
  (params (DeltaSeconds :type Float%20%28single-precision%29))
  (Transformation|SetActorLocation (+ (* (Variables|Default|GetDirection) (Variables|Default|GetSpeed)) (Transformation|GetActorLocation)) false false))

(event EventBeginPlay
  (Utilities|Time|SetTimerbyFunctionName 0 "Deactivate" 0.25))

(fn ConstructionScript)

(fn Deactivate
  (Components|Activation|Deactivate (Variables|Default|GetNiagara))
  (Utilities|Time|SetTimerbyFunctionName 0 "DestroySelf" 0.1))

(fn DestroySelf
  (Actor|DestroyActor))