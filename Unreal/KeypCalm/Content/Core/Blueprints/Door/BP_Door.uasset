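; BP_Door is a door that opens once when its matching grabbable prop is brought into its collision box.
; The overlapping BP_GrabProps must reference this door and have the required prop type.
; Opening plays a sound and a timeline that adds yaw to the mesh's starting world rotation, then prints a debug message.
; The construction script stores that rotation and picks door and border meshes plus door material from the door type.
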(event OnComponentBeginOverlap(BoxCollision)
  (params (OverlappedComponent :type Primitive%20Component%20Object%20Reference) (OtherActor :type Actor%20Object%20Reference) (OtherComp :type Primitive%20Component%20Object%20Reference) (OtherBodyIndex :type Integer) (bFromSweep :type Boolean) (SweepResult :type Hit%20Result%20Structure%20%28by%20ref%29))
  (bind _actualzrotation (Variables|Default|GetActualZRotation))
  (bind _asbp_grab_props (Utilities|Casting|CastToBP_GrabProps OtherActor))
  (if (and (== (Variables|/Game/Core/Blueprints/Props/BP_GrabProps.BP_GrabProps_C|GetDoorToOpen _asbp_grab_props) self) (Utilities|Enum|Equal(Enum) (Variables|/Game/Core/Blueprints/Props/BP_GrabProps.BP_GrabProps_C|GetPropType _asbp_grab_props) "NewEnumerator1"))
    (Utilities|FlowControl|DoOnce false
      (:Completed
        (Audio|PlaySound2D "/Game/Son/Bruitages/Doors/Open/OpenDoor_Cue.OpenDoor_Cue" 1.0 1.0 0.0 0 0)
        (bind _rotation (Timeline|RotateTheDoor Play)
          (:Update
            (Transformation|SetWorldRotation (Variables|Default|GetDoorMesh) (Math|Rotator|MakeRotator (.roll _actualzrotation) (.pitch _actualzrotation) (+ _rotation (.yaw _actualzrotation))) false false))
          (:Finished
            (Development|PrintString "Ouvert")))))))

(event EventBeginPlay)

(event Collision|EventActorBeginOverlap
  (params (OtherActor :type Actor%20Object%20Reference)))

(event EventTick
  (params (DeltaSeconds :type Float%20%28single-precision%29)))

(fn ConstructionScript
  (bind _doormesh (Variables|Default|GetDoorMesh))
  (bind _doormesh_2 (Variables|Default|GetDoorMesh))
  (Variables|Default|SetActualZRotation (Transformation|GetWorldRotation (Variables|Default|GetDoorMesh)))
  (switch Utilities|FlowControl|Switch|SwitchonPortes (Variables|Default|GetTypePorte)
    (:NewEnumerator0
      (Components|StaticMesh|SetStaticMesh _doormesh "/Game/Assets/Meshes/DOORS_WINDOWS/DOOR2/DOOR2_DOORMAIN2.DOOR2_DOORMAIN2")
      (Components|StaticMesh|SetStaticMesh (Variables|Default|Get%20) "/Game/Assets/Meshes/DOORS_WINDOWS/DOOR2/DOOR2_DOORborders2.DOOR2_DOORborders2")
      (Rendering|Material|SetMaterial _doormesh 0 "/Game/Assets/Meshes/DOORS_WINDOWS/DOOR2/M_DOOR_2.M_DOOR_2"))
    (:NewEnumerator1
      (Components|StaticMesh|SetStaticMesh _doormesh_2 "/Game/Assets/Meshes/DOORS_WINDOWS/DOOR1/DOOR1_DOORMAIN1.DOOR1_DOORMAIN1")
      (Components|StaticMesh|SetStaticMesh (Variables|Default|Get%20) "/Game/Assets/Meshes/DOORS_WINDOWS/DOOR1/DOOR1_DOORborders1.DOOR1_DOORborders1")
      (Rendering|Material|SetMaterial _doormesh_2 0 "/Game/Assets/Meshes/DOORS_WINDOWS/DOOR1/M_DOOR1.M_DOOR1"))))