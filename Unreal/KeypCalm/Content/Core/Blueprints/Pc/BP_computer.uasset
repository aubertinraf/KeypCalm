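; BP_computer is an interactable computer actor that opens an on-screen PC interface and can print out a prop.
; InteractAction blends the player camera to the computer over a short delay, then shows the WG_PC widget with UI-only input and a visible cursor.
; Print spawns a BP_GrabProps using StaticMesh1's relative location as the spawn location and prints a placeholder noise string.
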(event Custom|Print
  (Game|SpawnActorfromClass "/Game/Core/Blueprints/Props/BP_GrabProps.BP_GrabProps_C" (Math|Transform|MakeTransform (Variables|/Script/Engine.SceneComponent|GetRelativeLocation (Variables|Default|GetStaticMesh1)) "0, 0, 0" "1,1,1") "Undefined" 0 0)
  (Development|PrintString "*printNoises*"))

(event EventBeginPlay)

(event Collision|EventActorBeginOverlap
  (params (OtherActor :type Actor%20Object%20Reference)))

(event EventTick
  (params (DeltaSeconds :type Float%20%28single-precision%29)))

(event EventInteractAction
  (bind _returnvalue (Game|GetPlayerController 0))
  (Game|Player|SetViewTargetwithBlend (Game|GetPlayerController 0) self 1.0 "VTBlend_Linear" 0.0 false)
  (Utilities|FlowControl|Delay 1.0)
  (bind _returnvalue_2 (UserInterface|CreateWidget "/Game/Widgets/WG_PC.WG_PC_C"))
  (bind _output_get (Variables|Default|SetLeWidget _returnvalue_2))
  (UserInterface|Viewport|AddtoViewport _output_get 0)
  (Input|SetInputModeUIOnly _returnvalue _output_get "DoNotLock")
  (Variables|/Script/Engine.PlayerController|SetbShowMouseCursor _returnvalue true))

(fn ConstructionScript)