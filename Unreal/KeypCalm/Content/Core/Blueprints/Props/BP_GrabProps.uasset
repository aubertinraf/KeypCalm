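; Configurable grabbable prop that can be a key, a ladder or other object, with an optional destructible mesh.
; The construction script sets the static or destructible mesh, keeps keys non-simulated and titles them for door or lock; non-ladders lose their ladder collision at start.
; A destructible prop hit while grabbed breaks through radius damage, then drops.
; Dropped keys have physics switched off after a retriggerable delay.
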(event OnComponentHit(DestructibleMesh)
  (params (HitComponent :type Primitive%20Component%20Object%20Reference) (OtherActor :type Actor%20Object%20Reference) (OtherComp :type Primitive%20Component%20Object%20Reference) (NormalImpulse :type Vector :default "0, 0, 0") (Hit :type Hit%20Result%20Structure%20%28by%20ref%29))
  ;[1 1 1] Destructible?
  (if (and (Variables|Default|GetDestructible) (Variables|Default|GetGrabbed))
    (CallFunction|BreakProp)))

(event Custom|BreakProp
  (bind _destructiblemesh (Variables|Default|GetDestructibleMesh))
  ;[1 1 1] Applique damages au destructible mesh
  (Class|DestructibleComponent|ApplyRadiusDamage _destructiblemesh 1e+02 (Transformation|GetWorldLocation _destructiblemesh) 1e+02 1e+03 true)
  (Collision|SetCollisionEnabled _destructiblemesh "PhysicsOnly")
  (CallFunction|DropProp))

(event Custom|DropProp
  ;[1 1 1] Reset physics de la clé quand lâchée
  (switch Utilities|FlowControl|Switch|SwitchonPropEnum (Variables|Default|GetPropType)
    (:NewEnumerator1
      (Utilities|FlowControl|RetriggerableDelay 3.0)
      (Physics|SetSimulatePhysics (Variables|Default|GetStaticMesh) false))))

(event EventBeginPlay
  (bind _proptype (Variables|Default|GetPropType))
  ;[1 1 1] Begin Play
  (Utilities|FlowControl|Delay 0.2)
  (Utilities|FlowControl|Sequence
    (:then_0
      (switch Utilities|FlowControl|Switch|SwitchonPropEnum _proptype
        (:NewEnumerator1
          (Physics|SetSimulatePhysics (Variables|Default|GetStaticMesh) false))))
    (:then_1
      (if (Utilities|Enum|NotEqual(Enum) _proptype "NewEnumerator2")
        (Components|DestroyComponent (Variables|Default|GetLadderBoxCollision))))))

(fn ConstructionScript
  (bind _proptype (Variables|Default|GetPropType))
  (bind _staticmesh (Variables|Default|GetStaticMesh))
  (bind _returnvalue (Utilities|Enum|Equal(Enum) _proptype "NewEnumerator1"))
  (if (Variables|Default|GetDestructible)
    (Class|DestructibleComponent|SetDestructibleMesh (Variables|Default|GetDestructibleMesh) (Variables|Default|GetDestructibleVar))
    (else
      (Components|StaticMesh|SetStaticMesh _staticmesh (Variables|Default|GetStaticVar))
      (Physics|SetSimulatePhysics _staticmesh (select _returnvalue false true))
      ;[1 1 1] Set Key Name
      (if _returnvalue
        (if (Variables|Default|GetKeyDoor?)
          (Variables|Default|SetKeyTitle "Key Door")
          (else
            (Variables|Default|SetKeyTitle "Key Lock")))))))

(fn SetGrabbed
  (Variables|Default|SetGrabbed true))