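; BP_BouttonMenu is a walk-up main menu button built from a text render and a trigger box, used to load a level.
; BeginPlay sets the label, scales the box's width by TailleY and saves the original text color.
; Overlap by a ThirdPersonMainMenu stores that character and highlights the text; any end overlap clears both.
; The Action event opens the configured Level by name, with no caller in this graph.
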(event OnComponentBeginOverlap(Box)
  (params (OverlappedComponent :type Primitive%20Component%20Object%20Reference) (OtherActor :type Actor%20Object%20Reference) (OtherComp :type Primitive%20Component%20Object%20Reference) (OtherBodyIndex :type Integer) (bFromSweep :type Boolean) (SweepResult :type Hit%20Result%20Structure%20%28by%20ref%29))
  (bind _asthird_person_main_menu (Utilities|Casting|CastToThirdPersonMainMenu OtherActor))
  (Variables|Default|SetPerso _asthird_person_main_menu)
  (Rendering|Components|TextRender|SetTextRenderColor (Variables|Default|GetTextRender) (Variables|Default|GetColor)))

(event OnComponentEndOverlap(Box)
  (params (OverlappedComponent :type Primitive%20Component%20Object%20Reference) (OtherActor :type Actor%20Object%20Reference) (OtherComp :type Primitive%20Component%20Object%20Reference) (OtherBodyIndex :type Integer))
  (Variables|Default|SetPerso 0)
  (Rendering|Components|TextRender|SetTextRenderColor (Variables|Default|GetTextRender) (Variables|Default|GetMemColor)))

(event Custom|Action
  (Game|OpenLevel(byName) (Utilities|String|StringToName (Variables|Default|GetLevel))))

(event EventBeginPlay
  (bind _textrender (Variables|Default|GetTextRender))
  (Rendering|Components|TextRender|SetText _textrender (Utilities|Text|ToText(String) (Variables|Default|GetText)))
  (Transformation|SetRelativeScale3D (Variables|Default|GetBox) (Math|Vector|MakeVector 1.0 (Variables|Default|GetTaille%20y) 1.0))
  (Variables|Default|SetMemColor (Variables|/Script/Engine.TextRenderComponent|GetTextRenderColor _textrender)))

(event EventTick
  (params (DeltaSeconds :type Float%20%28single-precision%29)))

(fn ConstructionScript)