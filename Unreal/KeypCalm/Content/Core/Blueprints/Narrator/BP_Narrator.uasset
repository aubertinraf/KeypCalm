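; Narrator actor that plays random 2D voice lines to taunt the player and react to game events.
; On BeginPlay it registers itself with the ThirdPersonCharacter, and Talk routes each event type to its line picker.
; A retriggerable random delay fires idle taunts and restarts whenever a line is triggered.
; Taunts may draw a delayed Billy reply, thrown-prop lines play only occasionally, and the success line has no sounds assigned.
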(event Custom|Talk
  (params (Type :type NarratorEnum%20Enum :default "NewEnumerator0"))
  (switch Utilities|FlowControl|Switch|SwitchonNarratorEnum Type
    (:NewEnumerator0
      (CallFunction|RandomTauntFunc))
    (:NewEnumerator3
      (CallFunction|ThrowedPropFunc))
    (:NewEnumerator2
      (CallFunction|FoundKeyFunc))
    (:NewEnumerator1
      (CallFunction|SuccedFunc))))

(event Custom|ResetRandomDelay
  (Utilities|FlowControl|RetriggerableDelay (Math|Random|RandomFloatinRange 18.0 28.0))
  (CallFunction|Talk "NewEnumerator0"))

(event Custom|BillyRespound
  (Utilities|FlowControl|Delay (Math|Random|RandomFloatinRange 2.0 5.0))
  (if (== (Math|Random|RandomIntegerinRange 1 2) 1)
    (Audio|PlaySound2D (Utilities|Select :Index (Math|Random|RandomIntegerinRange 0 7) :Option%200 "/Game/Son/Voix/Billy/billy_voice_02.billy_voice_02" :Option%201 "/Game/Son/Voix/Billy/billy_voice_03.billy_voice_03" :Option%202 "/Game/Son/Voix/Billy/billy_voice_04.billy_voice_04" :Option%203 "/Game/Son/Voix/Billy/billy_voice_05.billy_voice_05" :Option%204 "/Game/Son/Voix/Billy/billy_voice_06.billy_voice_06" :Option%205 "/Game/Son/Voix/Billy/billy_voice_07.billy_voice_07" :Option%206 "/Game/Son/Voix/Billy/billy_groan_02.billy_groan_02" :Option%207 "/Game/Son/Voix/Billy/billy_groan_08.billy_groan_08") 1.0 1.0 0.0 0 0)))

(event EventBeginPlay
  (Utilities|FlowControl|Delay 0.2)
  (bind _returnvalue (Actor|GetActorOfClass "/Game/Core/Blueprints/TPC/ThirdPersonCharacter.ThirdPersonCharacter_C"))
  (Variables|/Game/Core/Blueprints/TPC/ThirdPersonCharacter.ThirdPersonCharacter_C|SetNarrator _returnvalue self)
  (Utilities|FlowControl|RetriggerableDelay (Math|Random|RandomFloatinRange 18.0 28.0))
  (CallFunction|Talk "NewEnumerator0"))

(fn ConstructionScript)

(fn RandomTauntFunc
  (Audio|PlaySound2D (Utilities|Select :Index (Math|Random|RandomIntegerinRange 0 24) :Option%200 "/Game/Son/Voix/Narrateur/Sans_reverb/Taunt_01.Taunt_01" :Option%201 "/Game/Son/Voix/Narrateur/Sans_reverb/Taunt_02.Taunt_02" :Option%202 "/Game/Son/Voix/Narrateur/Sans_reverb/Taunt_03.Taunt_03" :Option%203 "/Game/Son/Voix/Narrateur/Sans_reverb/Taunt_04.Taunt_04" :Option%204 "/Game/Son/Voix/Narrateur/Sans_reverb/Taunt_05.Taunt_05" :Option%205 "/Game/Son/Voix/Narrateur/Sans_reverb/Taunt_06.Taunt_06" :Option%206 "/Game/Son/Voix/Narrateur/Sans_reverb/Taunt_07.Taunt_07" :Option%207 "/Game/Son/Voix/Narrateur/Sans_reverb/Taunt_08.Taunt_08" :Option%208 "/Game/Son/Voix/Narrateur/Sans_reverb/Taunt_09.Taunt_09" :Option%209 "/Game/Son/Voix/Narrateur/Sans_reverb/Taunt_10.Taunt_10" :Option%2010 "/Game/Son/Voix/Narrateur/Sans_reverb/Taunt_12.Taunt_12" :Option%2011 "/Game/Son/Voix/Narrateur/Sans_reverb/Taunt_13.Taunt_13" :Option%2012 "/Game/Son/Voix/Narrateur/Sans_reverb/Taunt_14.Taunt_14" :Option%2013 0 :Option%2014 "/Game/Son/Voix/Narrateur/Sans_reverb/Taunt_15.Taunt_15" :Option%2015 "/Game/Son/Voix/Narrateur/Sans_reverb/Taunt_16.Taunt_16" :Option%2016 "/Game/Son/Voix/Narrateur/Sans_reverb/Taunt_17.Taunt_17" :Option%2017 "/Game/Son/Voix/Narrateur/Sans_reverb/Taunt_18.Taunt_18" :Option%2018 "/Game/Son/Voix/Narrateur/Sans_reverb/Taunt_19.Taunt_19" :Option%2019 "/Game/Son/Voix/Narrateur/Sans_reverb/Taunt_20.Taunt_20" :Option%2020 "/Game/Son/Voix/Narrateur/Sans_reverb/Taunt_21.Taunt_21" :Option%2021 "/Game/Son/Voix/Narrateur/Sans_reverb/Taunt_22.Taunt_22" :Option%2022 "/Game/Son/Voix/Narrateur/Sans_reverb/Taunt_23.Taunt_23" :Option%2023 "/Game/Son/Voix/Narrateur/Sans_reverb/Taunt_24.Taunt_24" :Option%2024 "/Game/Son/Voix/Narrateur/Sans_reverb/Taunt_25.Taunt_25") 1.0 1.0 0.0 0 0)
  (CallFunction|ResetRandomDelay)
  (CallFunction|BillyRespound))

(fn ThrowedPropFunc
  (if (== (Math|Random|RandomIntegerinRange 1 3) 3)
    (Audio|PlaySound2D (Utilities|Select :Index (Math|Random|RandomIntegerinRange 0 1) :Option%200 "/Game/Son/Voix/Narrateur/Sans_reverb/Throwed_01.Throwed_01" :Option%201 "/Game/Son/Voix/Narrateur/Sans_reverb/Throwed_02.Throwed_02") 1.0 1.0 0.0 0 0)
    (CallFunction|ResetRandomDelay)))

(fn FoundKeyFunc
  (Audio|PlaySound2D (Utilities|Select :Index (Math|Random|RandomIntegerinRange 0 1) :Option%200 "/Game/Son/Voix/Narrateur/Sans_reverb/FoundKey_01.FoundKey_01" :Option%201 "/Game/Son/Voix/Narrateur/Sans_reverb/FoundKey_02.FoundKey_02") 1.0 1.0 0.0 0 0)
  (CallFunction|ResetRandomDelay))

(fn SuccedFunc
  (Audio|PlaySound2D (Utilities|Select :Index (Math|Random|RandomIntegerinRange 0 1) :Option%200 0 :Option%201 0) 1.0 1.0 0.0 0 0)
  (CallFunction|ResetRandomDelay))