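; BP_SafeChest is a safe chest that accepts keys carried by the ThirdPersonCharacter and shows which locks are matched.
; BeginPlay gathers three lock components into a Locks array that is index-paired with the Keys array.
; On Box overlap, a carried key found in Keys turns the lock at that index green and is cleared from the character.
; No opening logic is present.
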(event OnComponentBeginOverlap(Box)
  (params (OverlappedComponent :type Primitive%20Component%20Object%20Reference) (OtherActor :type Actor%20Object%20Reference) (OtherComp :type Primitive%20Component%20Object%20Reference) (OtherBodyIndex :type Integer) (bFromSweep :type Boolean) (SweepResult :type Hit%20Result%20Structure%20%28by%20ref%29))
  (bind _asthird_person_character (Utilities|Casting|CastToThirdPersonCharacter OtherActor))
  (Utilities|IsValid (Variables|/Game/Core/Blueprints/TPC/ThirdPersonCharacter.ThirdPersonCharacter_C|GetKey _asthird_person_character)
    (:Is%20Valid
      (for (_array_element _array_index) (Variables|Default|GetKeys)
        (if (== (Variables|/Game/Core/Blueprints/TPC/ThirdPersonCharacter.ThirdPersonCharacter_C|GetKey _asthird_person_character) _array_element)
          (Rendering|Material|SetMaterial (Utilities|Array|Get(acopy) (Variables|Default|GetLocks) _array_index) 0 "/Engine/EngineDebugMaterials/VertexColorViewMode_GreenOnly.VertexColorViewMode_GreenOnly")
          (Variables|/Game/Core/Blueprints/TPC/ThirdPersonCharacter.ThirdPersonCharacter_C|SetKey _asthird_person_character 0))))))

(event EventBeginPlay
  (bind _locks (Variables|Default|GetLocks))
  (Utilities|Array|Add _locks (Variables|Default|GetLock_01))
  (Utilities|Array|Add _locks (Variables|Default|GetLock_02))
  (Utilities|Array|Add _locks (Variables|Default|GetLock_03)))

(fn ConstructionScript)